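; BP_Tunnel is a tunnel segment in an endless obstacle game, with a rotating wall mesh the player must avoid hitting.
; RandomizeWall picks a random hole mesh from the set for the given color and gives it a random roll.
; Reaching the trigger zone spawns the next tunnel, adds score, and destroys this segment with its health pack and enemy.
; Hitting the wall damages the player, shakes the camera and disables wall collision.
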(event OnComponentBeginOverlap(TriggerZone)
  (params (OverlappedComponent :type Primitive%20Component%20Object%20Reference) (OtherActor :type Actor%20Object%20Reference) (OtherComp :type Primitive%20Component%20Object%20Reference) (OtherBodyIndex :type Integer) (bFromSweep :type Boolean) (SweepResult :type Hit%20Result%20Structure%20%28by%20ref%29))
  (bind _enemy (Variables|Default|GetEnemy))
  (bind _health_pack (Variables|Default|GetHealth%20Pack))
  (bind _asbp_player (Utilities|Casting|CastToBP_Player OtherActor))
  (Default|SpawnTunnelatSpawnPoint (Variables|Default|GetTunnelSpawner))
  (Default|IncreaseScore _asbp_player)
  (Utilities|FlowControl|Sequence
    (:then_0
      (Utilities|IsValid _health_pack
        (:Is%20Valid
          (Actor|DestroyActor _health_pack))))
    (:then_1
      (Utilities|IsValid _enemy
        (:Is%20Valid
          (Actor|DestroyActor _enemy))))
    (:then_2
      (Actor|DestroyActor))))

(event OnComponentHit(WallMesh)
  (params (HitComponent :type Primitive%20Component%20Object%20Reference) (OtherActor :type Actor%20Object%20Reference) (OtherComp :type Primitive%20Component%20Object%20Reference) (NormalImpulse :type Vector :default "0, 0, 0") (Hit :type Hit%20Result%20Structure%20%28by%20ref%29))
  (Utilities|FlowControl|Sequence
    (:then_0
      (bind _asbp_player (Utilities|Casting|CastToBP_Player OtherActor))
      (Variables|Default|SetHit%20Wall true)
      (Default|DecreaseHealth _asbp_player)
      (Collision|SetCollisionProfileName (Variables|Default|GetWallMesh) "NoCollision" false :!class /Script/Engine.PrimitiveComponent)
      (Variables|/Game/InfiniteMatrix/Blueprints/BP_Player.BP_Player_C|SetShakeCamera? _asbp_player true))))

(event EventBeginPlay)

(event EventTick
  (params (DeltaSeconds :type Float%20%28single-precision%29))
  (Transformation|AddLocalRotation (Variables|Default|GetWallMesh) (Math|Rotator|MakeRotator (* DeltaSeconds (Variables|Default|GetRotateSpeed)) 0.0 0.0) false false))

(fn ConstructionScript)

(fn RandomizeWall
  (params (color :type Integer))
  (if (== color 0)
    (Components|StaticMesh|SetStaticMesh (Variables|Default|GetWallMesh) (Utilities|Select :Index (Math|Random|RandomIntegerinRange 0 3) :Option%200 "/Game/InfiniteMatrix/Meshes/SM_Hole_01.SM_Hole_01" :Option%201 "/Game/InfiniteMatrix/Meshes/SM_Hole_02.SM_Hole_02" :Option%202 "/Game/InfiniteMatrix/Meshes/SM_Hole_03.SM_Hole_03" :Option%203 "/Game/InfiniteMatrix/Meshes/SM_Hole_04.SM_Hole_04"))
    (Transformation|AddLocalRotation (Variables|Default|GetWallMesh) (Math|Rotator|MakeRotator (Math|Random|RandomFloatinRange 0.0 3.6e+02) 0.0 0.0) false false)
    (elif (== color 1)
      (Components|StaticMesh|SetStaticMesh (Variables|Default|GetWallMesh) (Utilities|Select :Index (Math|Random|RandomIntegerinRange 0 3) :Option%200 "/Game/InfiniteMatrix/Meshes/SM_Hole_05.SM_Hole_05" :Option%201 "/Game/InfiniteMatrix/Meshes/SM_Hole_06.SM_Hole_06" :Option%202 "/Game/InfiniteMatrix/Meshes/SM_Hole_07.SM_Hole_07" :Option%203 "/Game/InfiniteMatrix/Meshes/SM_Hole_08.SM_Hole_08"))
      (Transformation|AddLocalRotation (Variables|Default|GetWallMesh) (Math|Rotator|MakeRotator (Math|Random|RandomFloatinRange 0.0 3.6e+02) 0.0 0.0) false false)
      (else
        (Components|StaticMesh|SetStaticMesh (Variables|Default|GetWallMesh) (Utilities|Select :Index (Math|Random|RandomIntegerinRange 0 3) :Option%200 "/Game/InfiniteMatrix/Meshes/SM_Hole_09.SM_Hole_09" :Option%201 "/Game/InfiniteMatrix/Meshes/SM_Hole_10.SM_Hole_10" :Option%202 "/Game/InfiniteMatrix/Meshes/SM_Hole_11.SM_Hole_11" :Option%203 "/Game/InfiniteMatrix/Meshes/SM_Hole_12.SM_Hole_12"))
        (Transformation|AddLocalRotation (Variables|Default|GetWallMesh) (Math|Rotator|MakeRotator (Math|Random|RandomFloatinRange 0.0 3.6e+02) 0.0 0.0) false false)))))