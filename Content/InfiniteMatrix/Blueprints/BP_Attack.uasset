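; BP_Attack is a projectile actor that destroys enemies and scores points for the player.
; Tick moves it along world X at BulletSpeed, scaled by delta time.
; When its Bullet component hits a BP_Enemy, it destroys that enemy, sets the BP_Player pawn's hit message, increases the score and then destroys itself.
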(event OnComponentHit(bullet)
  (params (HitComponent :type Primitive%20Component%20Object%20Reference) (OtherActor :type Actor%20Object%20Reference) (OtherComp :type Primitive%20Component%20Object%20Reference) (NormalImpulse :type Vector :default "0, 0, 0") (Hit :type Hit%20Result%20Structure%20%28by%20ref%29))
  ;[1 1 1] Enemy Hit by bullet
  (bind _asbp_enemy (Utilities|Casting|CastToBP_Enemy OtherActor))
  (Actor|DestroyActor _asbp_enemy)
  (Utilities|FlowControl|Sequence
    (:then_0
      (bind _asbp_player (Utilities|Casting|CastToBP_Player (Game|Player|GetPlayerPawn 0)))
      (Variables|/Game/InfiniteMatrix/Blueprints/BP_Player.BP_Player_C|SetMessage _asbp_player "Hit Enemy")
      (Default|IncreaseScore _asbp_player))
    (:then_1
      (Actor|DestroyActor))))

(event EventBeginPlay)

(event Collision|EventActorBeginOverlap
  (params (OtherActor :type Actor%20Object%20Reference)))

(event EventTick
  (params (DeltaSeconds :type Float%20%28single-precision%29))
  ;[1 1 1] Make enemy move forward
  (Transformation|AddActorWorldOffset (Math|Vector|MakeVector (* DeltaSeconds (Variables|Default|GetBullet%20Speed)) 0.0 0.0)))

(fn ConstructionScript)