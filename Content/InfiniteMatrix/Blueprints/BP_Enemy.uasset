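; BP_Enemy is an enemy hazard that moves steadily and damages the player on contact.
; Each Tick offsets its Enemy component along negative local X at a constant speed, scaled by delta time.
; When that component hits a BP_Player, it calls DecreaseHealth, sets the player's hit message, destroys itself and sets the player's ShakeCamera flag.
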(event OnComponentHit(Enemy)
  (params (HitComponent :type Primitive%20Component%20Object%20Reference) (OtherActor :type Actor%20Object%20Reference) (OtherComp :type Primitive%20Component%20Object%20Reference) (NormalImpulse :type Vector :default "0, 0, 0") (Hit :type Hit%20Result%20Structure%20%28by%20ref%29))
  (bind _asbp_player (Utilities|Casting|CastToBP_Player OtherActor))
  (Default|DecreaseHealth _asbp_player)
  (Utilities|FlowControl|Sequence
    (:then_0
      (Variables|/Game/InfiniteMatrix/Blueprints/BP_Player.BP_Player_C|SetMessage _asbp_player "Hit Enemy, Health decreased by 10%")
      (Actor|DestroyActor))
    (:then_1
      (bind _asbp_player_2 (Utilities|Casting|CastToBP_Player OtherActor))
      (Variables|/Game/InfiniteMatrix/Blueprints/BP_Player.BP_Player_C|SetShakeCamera? _asbp_player_2 true))))

(event EventBeginPlay)

(event Collision|EventActorBeginOverlap
  (params (OtherActor :type Actor%20Object%20Reference)))

(event EventTick
  (params (DeltaSeconds :type Float%20%28single-precision%29))
  (Transformation|AddLocalOffset (Variables|Default|GetEnemy) (Math|Vector|MakeVector (* DeltaSeconds -1e+02) 0.0 0.0) false false))

(fn ConstructionScript)